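; Office desk with a locked drawer that opens a keypad widget and pauses the game when the player interacts nearby.
; A sphere overlap toggles input and a prompt widget, and cursor hover sets a material parameter on the desk.
; OpenDrawer, not called within this graph, slides the drawer by timeline with sound and advances the objective to the elevator.
; When the slide finishes, it marks the drawer open and briefly shows a keycard collection widget.
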(event OnComponentBeginOverlap(Sphere)
  (params (OverlappedComponent :type Primitive%20Component%20Object%20Reference) (OtherActor :type Actor%20Object%20Reference) (OtherComp :type Primitive%20Component%20Object%20Reference) (OtherBodyIndex :type Integer) (bFromSweep :type Boolean) (SweepResult :type Hit%20Result%20Structure%20%28by%20ref%29))
  (if (not (Variables|Default|GetIsOpen))
    (Input|EnableInput (Game|GetPlayerController 0))
    (Rendering|SetVisibility (Variables|Default|GetWidget) true false)))

(event OnComponentEndOverlap(Sphere)
  (params (OverlappedComponent :type Primitive%20Component%20Object%20Reference) (OtherActor :type Actor%20Object%20Reference) (OtherComp :type Primitive%20Component%20Object%20Reference) (OtherBodyIndex :type Integer))
  (Input|DisableInput (Game|GetPlayerController 0))
  (Rendering|SetVisibility (Variables|Default|GetWidget) false false))

(event OnBeginCursorOver(DeskComponent)
  (params (TouchedComponent :type Primitive%20Component%20Object%20Reference))
  (Rendering|Material|SetScalarParameterValueonMaterials (Variables|Default|GetDeskComponent) "B_1" 1.0))

(event OnEndCursorOver(DeskComponent)
  (params (TouchedComponent :type Primitive%20Component%20Object%20Reference))
  (Rendering|Material|SetScalarParameterValueonMaterials (Variables|Default|GetDeskComponent) "B_1" 0.0))

(event Custom|OpenDrawer
  (Utilities|FlowControl|Delay 0.5)
  (Audio|PlaySoundatLocation "/Game/group1/Audio_Group_1/A_DrawOpening_v01_T_Cue.A_DrawOpening_v01_T_Cue" "0, 0, 0" "0, 0, 0" 1.0 1.0 0.0 0 0 0)
  (bind _newtrack_0 (Timeline|DrawerAnimation Play)
    (:Update
      (Transformation|AddRelativeLocation (Variables|Default|GetDrawerMesh) (Math|Vector|MakeVector 0.0 (* (* (stale EventTick _output_get) 5.0) _newtrack_0) 0.0) false false)
      (bind _asfp_player_bp (Utilities|Casting|CastToFP_PlayerBP (stale OnComponentBeginOverlap(Sphere) OtherActor)))
      (bind _output_get (Variables|Default|SetObjective "Find a way into the drawer"))
      (if (Utilities|Enum|Equal(Enum) (Variables|/Game/General/Character/FP_PlayerBP.FP_PlayerBP_C|GetCurrent%20Objective _asfp_player_bp) _output_get)
        (Default|SlideOff _asfp_player_bp)
        (Variables|/Game/General/Character/FP_PlayerBP.FP_PlayerBP_C|SetCurrent%20Objective _asfp_player_bp "")
        (Audio|PlaySound2D "/Game/General/Audio/A_Notification_v01_G.A_Notification_v01_G" 1.0 1.0 0.0 0 0)
        (bind _asfp_player_bp_2 (Utilities|Casting|CastToFP_PlayerBP (stale OnComponentBeginOverlap(Sphere) OtherActor)))
        (if (Utilities|Enum|Equal(Enum) (Variables|/Game/General/Character/FP_PlayerBP.FP_PlayerBP_C|GetCurrent%20Objective _asfp_player_bp_2) "")
          (bind _output_get_2 (Variables|Default|SetNewObjective "Get to the elevator"))
          (Variables|/Game/General/Character/FP_PlayerBP.FP_PlayerBP_C|SetCurrent%20Objective _asfp_player_bp_2 _output_get_2)
          (Default|Slideon _asfp_player_bp_2)
          (Audio|PlaySound2D "/Game/General/Audio/A_Notification_v01_G.A_Notification_v01_G" 1.0 1.0 0.0 0 0))))
    (:Finished
      (Variables|Default|SetIsOpen true)
      (bind _returnvalue (UserInterface|CreateWidget "/Game/group1/GD_Group_1/Widgets/KeycardCollection_BP.KeycardCollection_BP_C" (Game|GetPlayerController 0)))
      (UserInterface|Viewport|AddtoViewport _returnvalue 0)
      (Utilities|FlowControl|Delay 2.0)
      (Widget|RemovefromParent _returnvalue)
      (Variables|/Script/Engine.PlayerController|SetbShowMouseCursor (Game|GetPlayerController 0) false))))

(event EventTick
  (params (DeltaSeconds :type Float%20%28single-precision%29))
  (bind _output_get (Variables|Default|SetDelta%20Seconds DeltaSeconds)))

(event EventBeginPlay
  (Rendering|SetVisibility (Variables|Default|GetWidget) false false)
  (bind _outactors (Actor|GetAllActorsOfClass "/Game/group1/GD_Group_1/Keycard_BP.Keycard_BP_C"))
  (Variables|Default|SetKeycard (Utilities|Array|Get(acopy) _outactors)))

(event Input|ActionEvents|InputActionInteract
  (params (Key :type Key%20Structure :default "None"))
  (:Pressed
    (Rendering|SetVisibility (Variables|Default|GetWidget) false false)
    (if (not (Variables|Default|GetIsOpen))
      (Rendering|SetVisibility (Variables|Default|GetWidget) false false)
      (Utilities|Casting|CastToFP_PlayerBP (stale OnComponentBeginOverlap(Sphere) OtherActor))
      (bind _returnvalue (UserInterface|CreateWidget "/Game/group1/GD_Group_1/Widgets/DrawerKeypad_BP.DrawerKeypad_BP_C"))
      (UserInterface|Viewport|AddtoViewport _returnvalue 0)
      (Game|SetGamePaused true)
      (Variables|/Script/Engine.PlayerController|SetbShowMouseCursor (Game|GetPlayerController 0) true))))

(fn ConstructionScript)
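; First-person player character handling movement, look, crouch, footstep audio, item pickup, inventory and pause menu.
; BeginPlay creates inventory and objective widgets, feeds the save game to the inventory and registers with FPMode.
; Pickup traces from the camera: tagged items go to inventory, some with popups or subtitles, while other movable meshes are carried by physics handle.
; A timeline resizes the crouch capsule, a looping timer plays footsteps, and noclip logic is unwired.
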(event Custom|OverlappedKeypad
  (params (Current%20Actor :type Actor%20Object%20Reference))
  (Variables|Default|SetCurrentKeypadActor Current%20Actor))

(event Custom|Footsteps%20Play
  ;[1 1 1] Footstep Audio (Sorry about the mess guys XD)
  (Audio|PlaySoundatLocation "/Game/General/Audio/A_Footsteps_v01_G_Cue.A_Footsteps_v01_G_Cue" (- (Transformation|GetActorLocation) "0, 0,44.000000") "0, 0, 0" 1.0 1.0 0.0 0 0 0))

(event Custom|Slide%20On
  ;[1 1 1] slide on and off animations for objectives
  (Default|Slideon (Variables|Default|GetObjectives%20widget%20ref)))

(event Custom|Slide%20Off
  ;[1 1 1] slide on and off animations for objectives
  (Default|SlideOff (Variables|Default|GetObjectives%20widget%20ref)))

(event EventBeginPlay
  ;[1 1 1] Inventory
  (Utilities|FlowControl|Sequence
    (:then_0
      (bind _asfp_player_controller (Utilities|Casting|CastToFP_PlayerController (Game|GetPlayerController 0)))
      (Variables|Default|SetPlayerControllerREF _asfp_player_controller)
      (bind _returnvalue (UserInterface|CreateWidget "/Game/General/UX/InventoryHUD/InventoryWidget_BP.InventoryWidget_BP_C"))
      (Variables|Default|SetInventory%20REF _returnvalue))
    (:then_1
      ;[1 1 1] Objective HUD
      (bind _returnvalue_2 (UserInterface|CreateWidget "/Game/General/UX/Objectives/W_ObjectiveWidget_v01_G.W_ObjectiveWidget_v01_G_C"))
      (bind _output_get (Variables|Default|SetObjectives%20Widget%20Ref _returnvalue_2))
      (UserInterface|Viewport|AddtoViewport _output_get 0))
    (:then_2
      (bind _asfpmode (Utilities|Casting|CastToFPMode (Game|GetGameMode)))
      (bind _savegame (Default|ReturnSaveGame _asfpmode))
      (Default|Start (Variables|Default|GetInventory%20REF) _savegame))
    (:then_3
      (Variables|/Script/Engine.PlayerController|SetbShowMouseCursor (Game|GetPlayerController 0) false))
    (:then_4
      (Default|PlayerRefGet _asfpmode self))))

(event EventTick
  (params (DeltaSeconds :type Float%20%28single-precision%29))
  (bind _returnvalue (Game|GetPlayerController 0))
  (bind (_sizex _sizey) (HUD|GetViewportSize _returnvalue))
  (Class|PlayerController|SetMouseLocation _returnvalue (/ _sizex 2) (/ _sizey 2)))

(event Input|ActionEvents|InputActionCrouch
  (params (Key :type Key%20Structure :default "None"))
  (bind _returnvalue (Transformation|GetActorLocation))
  ;[1 1 1] Crouch
  (:Pressed
    (bind _returnvalue_2 (Collision|LineTraceForObjects _returnvalue (+ (/ (* (Math|Vector|GetUpVector (Transformation|GetActorRotation)) 5e+03) (stale _capsuleheight)) _returnvalue) (Variables|Default|GetObject%20Types) false 0 "Persistent"))
    (if (not _returnvalue_2)
      (Utilities|FlowControl|FlipFlop
        (:A
          (bind _capsuleheight (Timeline|Timeline_0 Play)
            (:Update
              (Components|Capsule|SetCapsuleHalfHeight (Variables|Collision|GetCapsuleComponent) _capsuleheight true))))
        (:B
          (Timeline|Timeline_0 Reverse))))))

(event Input|ActionEvents|InputActionInventory
  (params (Key :type Key%20Structure :default "None"))
  ;[1 1 1] Inventory
  (:Pressed
    (Utilities|IsValid (Variables|Default|GetInventory%20REF)
      (:Is%20Valid
        (Game|SetGamePaused true)
        (Input|SetInputModeGameandUI (Variables|Default|GetPlayerControllerREF) (Variables|Default|GetHUD_REF) "DoNotLock" true)
        (Variables|/Script/Engine.PlayerController|SetbShowMouseCursor (Variables|Default|GetPlayerControllerREF) true)
        (UserInterface|Viewport|AddtoViewport (Variables|Default|GetInventory%20REF) 0)
        (Variables|Default|SetinventoryOpen true))
      (:Is%20Not%20Valid
        (Game|SetGamePaused true)
        (bind _returnvalue (UserInterface|CreateWidget "/Game/General/UX/InventoryHUD/InventoryWidget_BP.InventoryWidget_BP_C"))
        (Variables|Default|SetInventory%20REF _returnvalue)))))

(event Input|ActionEvents|InputActionPickup
  (params (Key :type Key%20Structure :default "None"))
  (bind _returnvalue (Game|GetPlayerController 0))
  (bind _returnvalue_2 (Game|GetPlayerController 0))
  (bind _returnvalue_3 (Game|GetPlayerController 0))
  (bind _fp_camera (Variables|Default|GetFP_Camera))
  (bind _inventory_ref (Variables|Default|GetInventory%20REF))
  (bind _returnvalue_4 (Transformation|GetWorldLocation _fp_camera))
  ;[1 1 1] Pickup
  (:Pressed
    (if (Variables|Default|GetHoldingItem)
      (Physics|Components|PhysicsHandle|ReleaseComponent (Variables|Default|GetPhysicsHandle))
      (Variables|Default|SetHoldingItem false)
      (else
        (bind (_outhit _returnvalue_5) (Collision|LineTraceByChannel _returnvalue_4 (+ (* (Math|Vector|GetForwardVector _fp_camera) 3e+02) _returnvalue_4) "TraceTypeQuery1" false 0 "None"))
        (if _returnvalue_5
          (Utilities|IsValid (.HitActor (Collision|BreakHitResult _outhit))
            (:Is%20Valid
              (bind _asstatic_mesh_component (Utilities|Casting|CastToStaticMeshComponent (.HitComponent (Collision|BreakHitResult _outhit))))
              (switch Utilities|FlowControl|Switch|SwitchonEComponentMobility (Variables|/Script/Engine.SceneComponent|GetMobility _asstatic_mesh_component)
                (:Movable
                  (switch name (Utilities|Array|Get(acopy) (Variables|/Script/Engine.Actor|GetTags (.HitActor (Collision|BreakHitResult _outhit))))
                    (:Default
                      (Physics|Components|PhysicsHandle|GrabComponentatLocationwithRotation (Variables|Default|GetPhysicsHandle) (.HitComponent (Collision|BreakHitResult _outhit)) "None" (Transformation|GetWorldLocation (.HitComponent (Collision|BreakHitResult _outhit))) "0, 0, 0")
                      (Variables|Default|SetHoldingItem (Utilities|IsValid (.HitActor (Collision|BreakHitResult _outhit)))))
                    (:NarrativeDocument
                      (Audio|PlaySoundatLocation "/Game/General/Audio/A_Keycard_v01_G_Cue.A_Keycard_v01_G_Cue" "0, 0, 0" "0, 0, 0" 1.0 1.0 0.0 0 0 0)
                      (Default|Item1 _inventory_ref)
                      (Actor|DestroyActor (.HitActor (Collision|BreakHitResult _outhit)) :!label _label))
                    (:Picture1
                      (Audio|PlaySoundatLocation "/Game/General/Audio/A_Keycard_v01_G_Cue.A_Keycard_v01_G_Cue" "0, 0, 0" "0, 0, 0" 1.0 1.0 0.0 0 0 0 :!label _label_2)
                      (CallFunction|PieceUp)
                      (Default|Item2 _inventory_ref)
                      (Actor|DestroyActor (.HitActor (Collision|BreakHitResult _outhit)))
                      (bind _returnvalue_6 (UserInterface|CreateWidget "/Game/group1/GD_Group_1/Widgets/W_TornPaper_v01_G.W_TornPaper_v01_G_C" _returnvalue_2))
                      (bind _returnvalue_7 (UserInterface|CreateWidget "/Game/group1/GD_Group_1/Widgets/W_inventoryitemTutorial_V01_GG.W_inventoryitemTutorial_V01_GG_C" _returnvalue_2))
                      (UserInterface|Viewport|AddtoViewport _returnvalue_7 0)
                      (Utilities|FlowControl|Delay 5.0)
                      (Widget|RemovefromParent _returnvalue_7))
                    (:Map
                      (Audio|PlaySoundatLocation "/Game/General/Audio/A_Keycard_v01_G_Cue.A_Keycard_v01_G_Cue" "0, 0, 0" "0, 0, 0" 1.0 1.0 0.0 0 0 0)
                      (Default|Item3 _inventory_ref)
                      (Actor|DestroyActor (.HitActor (Collision|BreakHitResult _outhit)))
                      ;[1 1 1] Map collection
                      (bind _returnvalue_8 (UserInterface|CreateWidget "/Game/group1/GD_Group_1/Widgets/MapCollection_BP.MapCollection_BP_C" _returnvalue_3))
                      (bind _returnvalue_9 (UserInterface|CreateWidget "/Game/group1/GD_Group_1/Widgets/W_inventoryitemTutorial_V01_GG.W_inventoryitemTutorial_V01_GG_C" _returnvalue_3))
                      (UserInterface|Viewport|AddtoViewport _returnvalue_8 0)
                      (Utilities|FlowControl|Delay 5.0)
                      (Widget|RemovefromParent _returnvalue_8)
                      ;[1 1 1] subtitle for map pickup
                      (Audio|PlaySound2D "/Game/group1/Audio_Group_1/VoiceActing/A_AudioTrackVA_v16_T.A_AudioTrackVA_v16_T" 1.0 1.0 0.0 0 0)
                      (bind _returnvalue_10 (UserInterface|CreateWidget "/Game/General/UX/Subtitles/W-SubtitleWidget_V01_G.W-SubtitleWidget_V01_G_C"))
                      (bind _output_get (Variables|Default|SetSubtitleWidgetRefrence _returnvalue_10))
                      (Default|DisplayLine _output_get "Benefactor \"Ugh looks like they split this code up Guess we will have took look around.\" ")
                      (UserInterface|Viewport|AddtoViewport _output_get 0)
                      (Utilities|FlowControl|Delay 3.5)
                      (Default|DisplayLine _output_get))
                    (:Pictograph
                      (Audio|PlaySoundatLocation "/Game/General/Audio/A_Keycard_v01_G_Cue.A_Keycard_v01_G_Cue" "0, 0, 0" "0, 0, 0" 1.0 1.0 0.0 0 0 0)
                      (Default|Item4 _inventory_ref)
                      ;[1 1 1] Map collection
                      (bind _returnvalue_11 (UserInterface|CreateWidget "/Game/group1/GD_Group_1/Widgets/PicCollection_BP1.PicCollection_BP1_C" _returnvalue))
                      (bind _returnvalue_12 (UserInterface|CreateWidget "/Game/group1/GD_Group_1/Widgets/W_inventoryitemTutorial_V01_GG.W_inventoryitemTutorial_V01_GG_C" _returnvalue))
                      (UserInterface|Viewport|AddtoViewport _returnvalue_11 0)
                      (bind _aspictograph (Utilities|Casting|CastToPictograph (.HitActor (Collision|BreakHitResult _outhit))))
                      (Actor|DestroyActor _aspictograph)
                      (Utilities|FlowControl|Delay 5.0)
                      (Widget|RemovefromParent _returnvalue_11))
                    (:Picture2
                      (goto _label_2))
                    (:Log1
                      (Audio|PlaySoundatLocation "/Game/General/Audio/A_Keycard_v01_G_Cue.A_Keycard_v01_G_Cue" "0, 0, 0" "0, 0, 0" 1.0 1.0 0.0 0 0 0)
                      (Default|Item6 _inventory_ref)
                      (goto _label))
                    (:Log2
                      (Audio|PlaySoundatLocation "/Game/General/Audio/A_Keycard_v01_G_Cue.A_Keycard_v01_G_Cue" "0, 0, 0" "0, 0, 0" 1.0 1.0 0.0 0 0 0)
                      (Default|Item7 _inventory_ref)
                      (goto _label))
                    (:Log3
                      (Audio|PlaySoundatLocation "/Game/General/Audio/A_Keycard_v01_G_Cue.A_Keycard_v01_G_Cue" "0, 0, 0" "0, 0, 0" 1.0 1.0 0.0 0 0 0)
                      (Default|Item8 _inventory_ref)
                      (goto _label))
                    (:Picture3
                      (goto _label_2))
                    (:Picture4
                      (goto _label_2))
                    (:Log4
                      (Default|Item5 _inventory_ref)
                      (goto _label))
                    (:ElementReport
                      (Audio|PlaySoundatLocation "/Game/General/Audio/A_Keycard_v01_G_Cue.A_Keycard_v01_G_Cue" "0, 0, 0" "0, 0, 0" 1.0 1.0 0.0 0 0 0)
                      (Default|Item9 _inventory_ref)
                      (goto _label))
                    (:Dagger
                      (Audio|PlaySoundatLocation "/Game/General/Audio/A_Keycard_v01_G_Cue.A_Keycard_v01_G_Cue" "0, 0, 0" "0, 0, 0" 1.0 1.0 0.0 0 0 0)
                      (Default|Item10 _inventory_ref)
                      (goto _label))))))))))))

(event Input|ActionEvents|InputActionPause
  (params (Key :type Key%20Structure :default "None"))
  (bind _returnvalue (Game|GetPlayerController 0))
  ;[1 1 1] Pause Menu
  (:Pressed
    (Utilities|IsValid (Variables|Default|GetPauseMenuREF)
      (:Is%20Valid
        _)
      (:Is%20Not%20Valid
        (bind _returnvalue_2 (UserInterface|CreateWidget "/Game/General/UX/PauseMenu/M_PauseMenuWidget_v01_G.M_PauseMenuWidget_v01_G_C"))
        (Variables|Default|SetPauseMenuREF _returnvalue_2)))
    (if (Game|IsGamePaused)
      (Widget|RemovefromParent (Variables|Default|GetPauseMenuREF))
      (bind _returnvalue_3 (Game|SetGamePaused false))
      (Variables|/Script/Engine.PlayerController|SetbShowMouseCursor _returnvalue _returnvalue_3)
      (Input|SetInputModeGameOnly _returnvalue)
      (else
        (UserInterface|Viewport|AddtoViewport (Variables|Default|GetPauseMenuREF) 0)
        (Game|SetGamePaused true)
        (Variables|/Script/Engine.PlayerController|SetbShowMouseCursor _returnvalue true)
        (Input|SetInputModeUIOnly _returnvalue (Variables|Default|GetPauseMenuREF) "LockInFullscreen")))))

(event Input|ActionEvents|InputActionGodMode
  (params (Key :type Key%20Structure :default "None"))
  ;[1 1 1] NoClip/Fly Note:Flying doesn't have horizontal motion, I don't know why.
)

(event Input|AxisEvents|InputAxisForward/Back
  (params (AxisValue :type Float%20%28single-precision%29))
  (bind _returnvalue (Transformation|GetVelocity))
  ;[1 1 1] Movement
  (Pawn|Input|AddMovementInput (Math|Vector|GetForwardVector (Math|Rotator|MakeRotator 0.0 0.0 (.Yaw (Math|Rotator|BreakRotator (Pawn|GetControlRotation :!class /Script/Engine.Pawn))))) AxisValue false)
  ;[1 1 1] Footstep Audio (Sorry about the mess guys XD)
  (if (and (Math|Boolean|ORBoolean (> (.x _returnvalue) 2.0) (< (.x _returnvalue) -2e+01) (> (.y _returnvalue) 2.0) (< (.y _returnvalue) -2e+01)) (== (.z _returnvalue) 0.0))
    (Utilities|FlowControl|DoOnce false :!label _label
      (:Completed
        (bind _returnvalue_2 (Utilities|Time|SetTimerbyEvent (delegate Custom|Footsteps%20Play) (Variables|Default|GetFootstepInterval) true))))
    (else
      (Utilities|Time|ClearandInvalidateTimerbyHandle _returnvalue_2)
      (goto _label Reset))))

(event Input|AxisEvents|InputAxisRight/Left
  (params (AxisValue :type Float%20%28single-precision%29))
  (bind _returnvalue (Transformation|GetVelocity))
  ;[1 1 1] Movement
  (Pawn|Input|AddMovementInput (Math|Vector|GetRightVector (Math|Rotator|MakeRotator 0.0 0.0 (.Yaw (Math|Rotator|BreakRotator (Pawn|GetControlRotation :!class /Script/Engine.Pawn))))) AxisValue false)
  ;[1 1 1] Footstep Audio (Sorry about the mess guys XD)
  (if (and (Math|Boolean|ORBoolean (> (.x _returnvalue) 2.0) (< (.x _returnvalue) -2e+01) (> (.y _returnvalue) 2.0) (< (.y _returnvalue) -2e+01)) (== (.z _returnvalue) 0.0))
    (Utilities|FlowControl|DoOnce false :!label _label
      (:Completed
        (bind _returnvalue_2 (Utilities|Time|SetTimerbyEvent (delegate Custom|Footsteps%20Play) (Variables|Default|GetFootstepInterval) true))))
    (else
      (Utilities|Time|ClearandInvalidateTimerbyHandle _returnvalue_2)
      (goto _label Reset))))

(event Input|AxisEvents|InputAxisLookXController
  (params (AxisValue :type Float%20%28single-precision%29))
  ;[1 1 1] Controller Look
  (Pawn|Input|AddControllerYawInput (* AxisValue (Variables|Default|GetContrrollerXRate) (Utilities|Time|GetWorldDeltaSeconds))))

(event Input|AxisEvents|InputAxisLookYController
  (params (AxisValue :type Float%20%28single-precision%29))
  ;[1 1 1] Controller Look
  (Pawn|Input|AddControllerPitchInput (* AxisValue (Variables|Default|GetControllerYRate) (Utilities|Time|GetWorldDeltaSeconds))))

(event Input|AxisEvents|InputAxisMouseY
  (params (AxisValue :type Float%20%28single-precision%29))
  (bind _fp_camera (Variables|Default|GetFP_Camera))
  ;[1 1 1] Looking
  (Pawn|Input|AddControllerPitchInput AxisValue)
  (Physics|Components|PhysicsHandle|SetTargetLocation (Variables|Default|GetPhysicsHandle) (+ (* (Math|Vector|GetForwardVector _fp_camera) 2e+02) (Transformation|GetWorldLocation _fp_camera))))

(event Input|AxisEvents|InputAxisMouseX
  (params (AxisValue :type Float%20%28single-precision%29))
  (bind _fp_camera (Variables|Default|GetFP_Camera))
  ;[1 1 1] Looking
  (Pawn|Input|AddControllerYawInput AxisValue)
  (Physics|Components|PhysicsHandle|SetTargetLocation (Variables|Default|GetPhysicsHandle) (+ (* (Math|Vector|GetForwardVector _fp_camera) 2e+02) (Transformation|GetWorldLocation _fp_camera))))

(fn ConstructionScript)

(fn CrouchAnim
  (params (bState :type Boolean))
  (if bState
    _))

(fn PieceUp
  (Variables|Default|SetNumberOfPieces (+ (Variables|Default|GetNumberOfPieces) 1)))